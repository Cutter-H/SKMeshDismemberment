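; BP_ExampleCharacter is a test character for a mannequin dismemberment component.
; Its only active logic prints the bone name when the component's OnBoneDismemberDelegate fires.
; Disconnected leftover chains would enable physics simulation after a delay, move the AI back and forth between two locations, and print neck bone health on authority.
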(event `self.ReceiveBeginPlay`)

(event `self.ReceiveTick`
  (params (DeltaSeconds :type "Float (single-precision)")))

(event `self.BP_MannequinDismemberment.OnBoneDismemberDelegate`
  (params (boneName :type Name) (disconnectionWorldLocation :type "Vector Structure") (damagingActors :type "Array of DismembermentDamageInstigator Structure (by ref)"))
  (`KismetSystemLibrary.PrintString` (`KismetStringLibrary.Conv_NameToString` boneName)))

(fn `UserConstructionScript`)