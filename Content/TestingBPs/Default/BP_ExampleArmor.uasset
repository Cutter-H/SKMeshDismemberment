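; BP_ExampleArmor is a test Blueprint for an armor dismemberment component, showing live bone health as debug text.
; On Tick, the authority loops over all bone health entries from BPArmorDismemberment and prints the neck_01 value with an index-based key.
; Unconnected leftover chains would enable physics simulation after a delay, or disable AI strafing and patrol endlessly between two location components.
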(event `self.ReceiveBeginPlay`)

(event `self.ReceiveTick`
  (params (DeltaSeconds :type "Float (single-precision)"))
  (`/Engine/EditorBlueprintResources/ActorMacros.Switch Has Authority`
    (:`Authority`
      (for (_array_element _array_index) (`SkeletalDismembermentMesh.GetAllBonesHealth` (`self.BP_ArmorDismemberment`))
        (if (== (break `BoneHealth` _array_element) "neck_01")
          (`KismetSystemLibrary.PrintString` (`KismetStringLibrary.Concat_StrStr` (`KismetStringLibrary.Conv_NameToString` (break `BoneHealth` _array_element)) ": " (`KismetStringLibrary.Conv_DoubleToString` (`.BoneHealth` (break `BoneHealth` _array_element)))) true true (struct :`G` 0.66 :`B` 1.0 :`A` 1.0) 2.0 (`KismetStringLibrary.Conv_StringToName` (`KismetStringLibrary.Conv_IntToString` (+ _array_index 100)))))))))

(fn `UserConstructionScript`)